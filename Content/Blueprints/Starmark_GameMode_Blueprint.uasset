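; Game mode for Starmark that handles player logins and the end of a multiplayer battle.
; PostLogin expects one player on DevLevel maps and two otherwise, then passes the cast controller to OnPlayerPostLogin.
; EndOfBattle waits briefly, destroys the online session and, on success, calls EndOfSession on every stored player controller.
; A DisplayErrorMessage helper prints error text on screen.
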(event EventPostLogin
  (params (NewPlayer :type Player%20Controller%20Object%20Reference))
  ;[1 1 1] Mtultiplayer Functions
  (bind _returnvalue (Game|GetCurrentLevelName true))
  (if (Utilities|String|Contains _returnvalue "DevLevel")
    (Variables|Default|SetExpectedPlayers 1)
    (else
      (Variables|Default|SetExpectedPlayers 2)))
  (bind _asplayer_controller_base_blueprint (Utilities|Casting|CastTo NewPlayer))
  (Class|StarmarkGameMode|OnPlayerPostLogin _asplayer_controller_base_blueprint))

(event EventEndOfBattle
  ;[1 1 1] Mtultiplayer Functions
  (Utilities|FlowControl|Delay 3.0)
  (|DestroySession (Game|GetPlayerController 0)
    (:OnSuccess
      (for _array_element (.PlayerControllerReferences (Variables|Default|GetPlayerControllerReferences))
        (bind _asplayer_controller_base_blueprint (Utilities|Casting|CastTo _array_element))
        (CallFunction|EndOfSession _asplayer_controller_base_blueprint)))))

(fn ConstructionScript)