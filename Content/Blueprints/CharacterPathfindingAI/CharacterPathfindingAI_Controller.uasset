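; AI controller for grid-based characters that runs the pathfinding behavior tree on possess and replicates movement.
; It binds to move completion and, for any valid result, refreshes the state of every grid tile actor.
; It then has every entity character recompute the tiles it occupies by size, finding both sets with world-wide actor searches.
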(event Custom|ReceiveMoveCompleted_Event
  (params (RequestID :type AI%20Request%20ID%20Structure) (Result :type EPathFollowingResult%20Enum :default "Success"))
  ;[1 1 1] Update GridTiles upon Avatars finishing movement
  (if (Utilities|Enum|NotEqual(Enum) Result "Invalid")
    (bind _outactors (Actor|GetAllActorsOfClass "/Game/Blueprints/Actor_GridTile_Blueprint.Actor_GridTile_Blueprint_C"))
    (for _array_element _outactors
      (Class|ActorGridTile|UpdateGridTileState _array_element))
    (bind _outactors_2 (Actor|GetAllActorsOfClass "/Game/Blueprints/Character_Entity_Blueprint.Character_Entity_Blueprint_C"))
    (for _array_element_2 _outactors_2
      (Class|CharacterPathfinder|SetTilesOccupiedbySize _array_element_2 false))))

(event EventPossess
  (params (PossessedPawn :type Pawn%20Object%20Reference))
  ;[1 1 1] Run the AI Pathfinding BehaviourTree
  (AI|RunBehaviorTree "/Game/Blueprints/CharacterPathfindingAI/CharacterPathfindingAI_BehaviourTree.CharacterPathfindingAI_BehaviourTree")
  (Class|Actor|SetReplicateMovement true)
  (EventDispatchers|AssignReceiveMoveCompleted (delegate Custom|ReceiveMoveCompleted_Event)))

(fn ConstructionScript)