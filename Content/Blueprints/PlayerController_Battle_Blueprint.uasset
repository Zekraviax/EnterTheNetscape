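; Battle player controller for a grid-based tactics game, handling cursor hover, avatar facing and click commands for the selected avatar.
; Tick snaps avatar yaw toward the mouse or movement direction and notifies the hovered tile.
; Hover highlights either the navigation path, colored by movement budget with free stone roads, or attack-pattern tiles.
; Left click passes attack-trace overlaps as targets; right click sends a move command, trimming the path before the AI controller moves.
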(event Custom|GridTileHoverDrawPath
  (params (GridTileLocation :type Vector))
  (bind _tilehighlightmode (Variables|Default|GetTileHighlightMode))
  (bind _currentselectedavatar (Variables|Default|GetCurrentSelectedAvatar))
  ;[1 1 1] Mouse Functions
  (bind _output_get (Variables|Default|SetCursorLocationSnappedToGrid GridTileLocation))
  (bind _outactors (Actor|GetAllActorsOfClass "/Game/Blueprints/Actor_AttackEffectsLibrary_Blueprint.Actor_AttackEffectsLibrary_Blueprint_C"))
  (if (> (Utilities|Array|Length _outactors) 0)
    (bind _outactors_2 (Actor|GetAllActorsOfClass "/Game/Blueprints/Actor_WorldGrid_Blueprint.Actor_WorldGrid_Blueprint_C"))
    (bind _outactors_3 (Actor|GetAllActorsOfClass "/Game/Blueprints/Actor_GridTile_Blueprint.Actor_GridTile_Blueprint_C"))
    (for _array_element _outactors_3
      (if (Class|KismetMathLibrary|EqualIntPointIntPoint (.GridPos (Class|ActorWorldGrid|ConvertWorldTiletoGridCoordinates (Utilities|Array|Get(acopy) _outactors_2) (Transformation|GetActorLocation _array_element))) (.GridPos (Class|ActorWorldGrid|ConvertWorldTiletoGridCoordinates (Utilities|Array|Get(acopy) _outactors_2) GridTileLocation)))
        (Class|ActorGridTile|SetTileHighlightProperties _array_element true false "WithinAttackRange")
        (else
          (Class|ActorGridTile|SetTileHighlightProperties _array_element true true "Normal"))))
    (else
      (Utilities|IsValid _currentselectedavatar
        (:Is%20Valid
          (if (Utilities|Enum|Equal(Enum) _tilehighlightmode "E_MovePath")
            (bind _returnvalue (Class|NavigationSystemV1|FindPathtoLocationSynchronously (Transformation|GetWorldLocation (Variables|/Script/Engine.Character|GetMesh _currentselectedavatar)) _output_get (.AsCharacter%20Pathfinding%20AI%20Controller (Utilities|Casting|CastToCharacterPathfindingAI_Controller (Pawn|GetController _currentselectedavatar))) 0))
            (Utilities|Array|Clear (Variables|Default|GetGridTilesOnHoverPath))
            (bind _outactors_4 (Actor|GetAllActorsOfClass "/Game/Blueprints/Actor_GridTile_Blueprint.Actor_GridTile_Blueprint_C"))
            (for _array_element_2 _outactors_4
              (Class|ActorGridTile|SetTileHighlightProperties _array_element_2 false true "Normal"))
            (Utilities|IsValid _returnvalue
              (:Is%20Valid
                (bind _outactors_5 (Actor|GetAllActorsOfClass "/Game/Blueprints/Actor_WorldGrid_Blueprint.Actor_WorldGrid_Blueprint_C"))
                (for _array_element_3 (Variables|/Script/NavigationSystem.NavigationPath|GetPathPoints _returnvalue)
                  (for _array_element_4 _outactors_4
                    (if (Class|KismetMathLibrary|EqualIntPointIntPoint (.GridPos (Class|ActorWorldGrid|ConvertWorldTiletoGridCoordinates (Utilities|Array|Get(acopy) _outactors_5) (Transformation|GetActorLocation _array_element_4))) (.GridPos (Class|ActorWorldGrid|ConvertWorldTiletoGridCoordinates (Utilities|Array|Get(acopy) _outactors_5) _array_element_3)))
                      (Utilities|Array|Add (Variables|Default|GetGridTilesOnHoverPath) _array_element_4))))
                (Variables|Default|SetAvatarCurrentTileMoves (Utilities|Struct|BreakNetscapeExplorer_Struct (Variables|/Script/Starmark.Character_Pathfinder|GetAvatarData (Variables|Default|GetCurrentSelectedAvatar))))
                (for (_array_element_5 _array_index) (Variables|Default|GetGridTilesOnHoverPath)
                  (if (> _array_index 0)
                    (bind _output_get_2 (Variables|Default|SetLocalTileMovementCost (Variables|/Script/Starmark.Actor_GridTile|GetMovementCost _array_element_5)))
                    (if (Utilities|Array|ContainsItem (Variables|/Script/Starmark.Actor_GridTile|GetProperties _array_element_5) "E_StoneRoad")
                      (Variables|Default|SetLocalTileMovementCost 0))
                    (if (> _output_get_2 (Variables|Default|GetAvatarCurrentTileMoves))
                      (Class|ActorGridTile|SetTileHighlightProperties _array_element_5 true true "OnMouseHoverTileUnreachable")
                      (else
                        (Class|ActorGridTile|SetTileHighlightProperties _array_element_5 true true "OnMouseHover")))
                    (Variables|Default|SetAvatarCurrentTileMoves (- (Variables|Default|GetAvatarCurrentTileMoves) _output_get_2))))))
            (elif (Utilities|Enum|Equal(Enum) _tilehighlightmode "E_AttackPattern")
              (Utilities|Array|Clear (Variables|Default|GetGridTilesOnHoverPath))
              (bind _outactors_6 (Actor|GetAllActorsOfClass "/Game/Blueprints/Actor_GridTile_Blueprint.Actor_GridTile_Blueprint_C"))
              (for _array_element_6 _outactors_6
                (Class|ActorGridTile|SetTileHighlightProperties _array_element_6 false true "Normal"))
              (for _array_element_7 (Collision|GetOverlappingActors (Variables|/Script/Starmark.Character_Pathfinder|GetAttackTraceActor (Variables|Default|GetCurrentSelectedAvatar)) "/Game/Blueprints/Actor_GridTile_Blueprint.Actor_GridTile_Blueprint_C" :!class /Script/Engine.PrimitiveComponent)
                (bind _asactor_grid_tile_blueprint (Utilities|Casting|CastToActor_GridTile_Blueprint _array_element_7))
                (Class|ActorGridTile|SetTileHighlightProperties _asactor_grid_tile_blueprint true false "WithinAttackRange")))))))))

(event Custom|GetCursorOverTile
  (bind _asactor_grid_tile_blueprint (Utilities|Casting|CastToActor_GridTile_Blueprint (.HitActor (Collision|BreakHitResult (.HitResult (Game|Player|GetHitResultUnderCursorbyChannel "TraceTypeQuery1" true))))))
  (Default|ManualBeginCursorOver _asactor_grid_tile_blueprint))

(event Custom|GetMoveCommand_Server
  (params (Location :type Vector))
  (bind _currentselectedavatar (Variables|Default|GetCurrentSelectedAvatar))
  (bind _returnvalue (Pawn|GetController _currentselectedavatar))
  (bind _ascharacter_pathfinding_ai_controller (Utilities|Casting|CastToCharacterPathfindingAI_Controller _returnvalue))
  ;[1 1 1] Mouse Functions
  (bind _returnvalue_2 (Class|NavigationSystemV1|FindPathtoLocationSynchronously (Transformation|GetWorldLocation (Variables|/Script/Engine.Character|GetMesh _currentselectedavatar)) Location _ascharacter_pathfinding_ai_controller 0))
  (if (and (Utilities|IsValid _returnvalue_2) (> (Utilities|Array|Length (Variables|/Script/NavigationSystem.NavigationPath|GetPathPoints _returnvalue_2)) 0))
    (while (> (- (Utilities|Array|Length (Variables|/Script/NavigationSystem.NavigationPath|GetPathPoints _returnvalue_2)) 1) (.CurrentTileMoves (Utilities|Struct|BreakNetscapeExplorer_Struct (Variables|/Script/Starmark.Character_Pathfinder|GetAvatarData _currentselectedavatar))))
      (Utilities|Array|RemoveIndex (Variables|/Script/NavigationSystem.NavigationPath|GetPathPoints _returnvalue_2) (- (Utilities|Array|Length (Variables|/Script/NavigationSystem.NavigationPath|GetPathPoints _returnvalue_2)) 1)))
    (AI|Navigation|MovetoLocation _ascharacter_pathfinding_ai_controller (Utilities|Array|Get(acopy) (Variables|/Script/NavigationSystem.NavigationPath|GetPathPoints _returnvalue_2) (- (Utilities|Array|Length (Variables|/Script/NavigationSystem.NavigationPath|GetPathPoints _returnvalue_2)) 1)) -1.0 false true false true 0)
    (Class|AIControllerAvatar|GetMoveCommandfromPlayer _ascharacter_pathfinding_ai_controller (Utilities|Array|Get(acopy) (Variables|/Script/NavigationSystem.NavigationPath|GetPathPoints _returnvalue_2) (- (Utilities|Array|Length (Variables|/Script/NavigationSystem.NavigationPath|GetPathPoints _returnvalue_2)) 1)) (Math|Float|Round (Class|NavigationPath|GetPathCost _returnvalue_2)) _currentselectedavatar)
    (bind _outactors (Actor|GetAllActorsOfClass "/Game/Blueprints/Actor_GridTile_Blueprint.Actor_GridTile_Blueprint_C"))
    (for _array_element (Variables|/Script/NavigationSystem.NavigationPath|GetPathPoints _returnvalue_2)
      (for _array_element_2 _outactors
        (if (Math|Vector|Equal(Vector) (Transformation|GetActorLocation _array_element_2) _array_element 1.0)
          (Utilities|Array|Add (Variables|/Script/Starmark.Character_Pathfinder|GetCurrentPathTiles (Variables|Default|GetCurrentSelectedAvatar)) _array_element_2))))
    (else
      (Development|PrintText "Error: No Points in Path" true true "(R=1.000000,G=0.000000,B=0.000000,A=1.000000)" 15.0))))

(event Custom|EndOfSession
  ;[1 1 1] Multiplyer Function(s)
  (Viewport|RemoveAllWidgets)
  (Game|OpenLevel(byName) "MainMenu"))

(event EventBeginPlay
  (Input|SetInputModeGameandUI self 0 "DoNotLock" false))

(event EventTick
  (params (DeltaSeconds :type Float%20%28single-precision%29))
  (bind (_worldlocation _worlddirection) (Game|Player|ConvertMouseLocationToWorldSpace))
  (bind _returnvalue (Math|Conversions|ToFloat(Integer) 90))
  (bind _currentselectedavatar (Variables|Default|GetCurrentSelectedAvatar))
  (bind _currentselectedavatar_2 (Variables|Default|GetCurrentSelectedAvatar))
  (bind _returnvalue_2 (Transformation|GetVelocity _currentselectedavatar))
  (bind _attackrotationsnaptodegrees (Variables|/Script/Starmark.Character_Pathfinder|GetAttackRotationSnapToDegrees _currentselectedavatar_2))
  (bind _returnvalue_3 (Math|Conversions|ToFloat(Integer) _attackrotationsnaptodegrees))
  ;[1 1 1] Rotate current avatar towards mouse/towards path
  (Utilities|IsValid _currentselectedavatar_2
    (:Is%20Valid
      (CallFunction|GetCursorOverTile)
      (if (Variables|/Script/Starmark.Character_Pathfinder|GetRotateAvatarTowardsMouse _currentselectedavatar_2)
        (Transformation|SetActorRotation _currentselectedavatar_2 (Math|Rotator|MakeRotator 0.0 0.0 (* (Math|Float|Round (/ (.Yaw (Math|Rotator|BreakRotator (Math|Rotator|FindLookatRotation (Transformation|GetActorLocation _currentselectedavatar_2) (+ _worldlocation (* (* _worlddirection (/ (.Z (Math|Vector|BreakVector _worldlocation)) (.Z (Math|Vector|BreakVector _worlddirection)))) -1.0))))) _returnvalue_3)) _returnvalue_3)) true)
        (else
          ;;[1 1 1] Avatar Instant Rotation (when moving)
          (if (> (Math|Vector|VectorLength _returnvalue_2) 0.0)
            (Transformation|SetActorRotation _currentselectedavatar (Math|Rotator|MakeRotator 0.0 0.0 (* (Math|Float|Round (/ (.Yaw (Math|Rotator|BreakRotator (Math|Conversions|RotationFromXVector _returnvalue_2))) _returnvalue)) _returnvalue)) true)))))))

(event Input|ActionEvents|InputActionLeftMouseButtonDown
  (params (Key :type Key%20Structure :default "None"))
  (bind _currentselectedavatar (Variables|Default|GetCurrentSelectedAvatar))
  (bind _attacktraceactor (Variables|/Script/Starmark.Character_Pathfinder|GetAttackTraceActor _currentselectedavatar))
  (bind _validattacktargetsarray (Variables|/Script/Starmark.Character_Pathfinder|GetValidAttackTargetsArray _currentselectedavatar))
  (bind _overlappingactors (Collision|GetOverlappingActors _attacktraceactor 0 :!class /Script/Engine.PrimitiveComponent))
  ;[1 1 1] Mouse Functions
  (:Released
    (if (Variables|Default|GetIsCurrentlyActingPlayer)
      (Utilities|Array|Clear _validattacktargetsarray)
      (for _array_element _overlappingactors
        (Utilities|Array|Add _validattacktargetsarray _array_element))
      (Class|PlayerControllerBattle|OnPrimaryClick (.HitActor (Collision|BreakHitResult (.HitResult (Game|Player|GetHitResultUnderCursorbyChannel "TraceTypeQuery1" true)))) _overlappingactors)
      (Variables|/Script/Starmark.Character_Pathfinder|SetRotateAvatarTowardsMouse (Variables|Default|GetCurrentSelectedAvatar) false)
      (Variables|Default|SetTileHighlightMode "E_MovePath"))))

(event Input|ActionEvents|InputActionRightMouseButtonDown
  (params (Key :type Key%20Structure :default "None"))
  (bind _hitresult (Game|Player|GetHitResultUnderCursorbyChannel "TraceTypeQuery1" true))
  (bind _hitactor (Collision|BreakHitResult _hitresult))
  ;[1 1 1] Mouse Functions
  (:Released
    (if (Variables|Default|GetIsCurrentlyActingPlayer)
      (Utilities|IsValid _hitactor
        (:Is%20Valid
          (CallFunction|GetMoveCommandServer (Transformation|GetActorLocation _hitactor)))
        (:Is%20Not%20Valid
          _))
      (Variables|/Script/Starmark.Character_Pathfinder|SetRotateAvatarTowardsMouse (Variables|Default|GetCurrentSelectedAvatar) false)
      (Variables|Default|SetTileHighlightMode "E_MovePath"))))

(fn ConstructionScript)