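; Base character for a grid-tactics avatar, handling tile-by-tile movement effects, attack-range highlighting and a spinning selection ring.
; While moving, each path tile triggers once, applying Burning damage, then either adding Burning from a data table on Fire tiles or spending a move.
; An attack trace collider follows the grid-snapped cursor, and trace overlaps recolour tiles for non-Ring attacks according to the controller's highlight mode.
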(event OnComponentBeginOverlap(BoxComponent)
  (params (OverlappedComponent :type Primitive%20Component%20Object%20Reference) (OtherActor :type Actor%20Object%20Reference) (OtherComp :type Primitive%20Component%20Object%20Reference) (OtherBodyIndex :type Integer) (bFromSweep :type Boolean) (SweepResult :type Hit%20Result%20Structure%20%28by%20ref%29))
  (bind _currentpathtiles (Variables|Default|GetCurrentPathTiles))
  (bind _asactor_grid_tile_blueprint (Utilities|Casting|CastToActor_GridTile_Blueprint OtherActor))
  (Utilities|Casting|CastToBoxComponent OverlappedComponent)
  (if (and (> (Math|Vector|VectorLength (Transformation|GetVelocity)) 0.0) (Utilities|Array|ContainsItem _currentpathtiles _asactor_grid_tile_blueprint))
    (CallFunction|BeginTileOverlap _asactor_grid_tile_blueprint)
    (Utilities|Array|RemoveItem _currentpathtiles _asactor_grid_tile_blueprint)))

(event OnComponentBeginOverlap(AttackTraceCollisionComponent)
  (params (OverlappedComponent :type Primitive%20Component%20Object%20Reference) (OtherActor :type Actor%20Object%20Reference) (OtherComp :type Primitive%20Component%20Object%20Reference) (OtherBodyIndex :type Integer) (bFromSweep :type Boolean) (SweepResult :type Hit%20Result%20Structure%20%28by%20ref%29))
  (bind _playercontrollerreference (Variables|Default|GetPlayerControllerReference))
  ;[1 1 1] Attack Trace Actors
  (Utilities|IsValid (Variables|Default|GetPlayerControllerReference)
    (:Is%20Valid
      (if (and (Utilities|Enum|Equal(Enum) (Variables|/Script/Starmark.PlayerController_Battle|GetTileHighlightMode _playercontrollerreference) "E_None") (not (Utilities|Enum|Equal(Enum) (Utilities|Struct|BreakAvatar_AttackStruct (Variables|/Script/Starmark.Character_Pathfinder|GetCurrentSelectedAttack (Variables|/Script/Starmark.PlayerController_Battle|GetCurrentSelectedAvatar _playercontrollerreference))) "Ring")))
        (bind _asactor_grid_tile_blueprint (Utilities|Casting|CastToActor_GridTile_Blueprint (stale OnComponentBeginOverlap(AttackTraceActor) OtherActor)))
        (Variables|/Script/Starmark.Actor_GridTile|SetChangeColourOnMouseHover _asactor_grid_tile_blueprint false)
        (Class|ActorGridTile|UpdateTileColour _asactor_grid_tile_blueprint "WithinAttackRange")))))

(event OnComponentEndOverlap(AttackTraceCollisionComponent)
  (params (OverlappedComponent :type Primitive%20Component%20Object%20Reference) (OtherActor :type Actor%20Object%20Reference) (OtherComp :type Primitive%20Component%20Object%20Reference) (OtherBodyIndex :type Integer))
  (bind _playercontrollerreference (Variables|Default|GetPlayerControllerReference))
  ;[1 1 1] Attack Trace Actors
  (Utilities|IsValid 0
    (:Is%20Valid
      (if (and (Utilities|Enum|Equal(Enum) (Variables|/Script/Starmark.PlayerController_Battle|GetTileHighlightMode _playercontrollerreference) "E_AttackPattern") (not (Utilities|Enum|Equal(Enum) (Utilities|Struct|BreakAvatar_AttackStruct (Variables|/Script/Starmark.Character_Pathfinder|GetCurrentSelectedAttack (Variables|/Script/Starmark.PlayerController_Battle|GetCurrentSelectedAvatar _playercontrollerreference))) "Ring")))
        (bind _asactor_grid_tile_blueprint (Utilities|Casting|CastToActor_GridTile_Blueprint (stale OnComponentEndOverlap(AttackTraceActor) OtherActor)))
        (Variables|/Script/Starmark.Actor_GridTile|SetChangeColourOnMouseHover _asactor_grid_tile_blueprint true)
        (Class|ActorGridTile|UpdateTileColour _asactor_grid_tile_blueprint "Normal")))))

(event OnComponentBeginOverlap(AttackTraceActor)
  (params (OverlappedComponent :type Primitive%20Component%20Object%20Reference) (OtherActor :type Actor%20Object%20Reference) (OtherComp :type Primitive%20Component%20Object%20Reference) (OtherBodyIndex :type Integer) (bFromSweep :type Boolean) (SweepResult :type Hit%20Result%20Structure%20%28by%20ref%29))
  (bind _playercontrollerreference (Variables|Default|GetPlayerControllerReference))
  ;[1 1 1] Attack Trace Actors
  (Utilities|IsValid (Variables|Default|GetPlayerControllerReference)
    (:Is%20Valid
      (if (and (Utilities|Enum|Equal(Enum) (Variables|/Script/Starmark.PlayerController_Battle|GetTileHighlightMode _playercontrollerreference) "E_None") (not (Utilities|Enum|Equal(Enum) (Utilities|Struct|BreakAvatar_AttackStruct (Variables|/Script/Starmark.Character_Pathfinder|GetCurrentSelectedAttack (Variables|/Script/Starmark.PlayerController_Battle|GetCurrentSelectedAvatar _playercontrollerreference))) "Ring")))
        (bind _asactor_grid_tile_blueprint (Utilities|Casting|CastToActor_GridTile_Blueprint OtherActor))
        (Variables|/Script/Starmark.Actor_GridTile|SetChangeColourOnMouseHover _asactor_grid_tile_blueprint false)
        (Class|ActorGridTile|UpdateTileColour _asactor_grid_tile_blueprint "WithinAttackRange")))))

(event OnComponentEndOverlap(AttackTraceActor)
  (params (OverlappedComponent :type Primitive%20Component%20Object%20Reference) (OtherActor :type Actor%20Object%20Reference) (OtherComp :type Primitive%20Component%20Object%20Reference) (OtherBodyIndex :type Integer))
  (bind _playercontrollerreference (Variables|Default|GetPlayerControllerReference))
  ;[1 1 1] Attack Trace Actors
  (Utilities|IsValid 0
    (:Is%20Valid
      (if (and (Utilities|Enum|Equal(Enum) (Variables|/Script/Starmark.PlayerController_Battle|GetTileHighlightMode _playercontrollerreference) "E_AttackPattern") (not (Utilities|Enum|Equal(Enum) (Utilities|Struct|BreakAvatar_AttackStruct (Variables|/Script/Starmark.Character_Pathfinder|GetCurrentSelectedAttack (Variables|/Script/Starmark.PlayerController_Battle|GetCurrentSelectedAvatar _playercontrollerreference))) "Ring")))
        (bind _asactor_grid_tile_blueprint (Utilities|Casting|CastToActor_GridTile_Blueprint OtherActor))
        (Variables|/Script/Starmark.Actor_GridTile|SetChangeColourOnMouseHover _asactor_grid_tile_blueprint true)
        (Class|ActorGridTile|UpdateTileColour _asactor_grid_tile_blueprint "Normal")))))

(event OnBeginCursorOver(BoxComponents)
  (params (TouchedComponent :type Primitive%20Component%20Object%20Reference))
  (Class|CharacterPathfinder|OnAvatarCursorOverBegin))

(event Custom|BeginTileOverlap
  (params (GridTileReference :type Actor%20Grid%20Tile%20Blueprint%20Object%20Reference))
  (for _array_element (Variables|Default|GetCurrentStatusEffectsArray)
    (if (Utilities|String|Contains (Utilities|Struct|BreakAvatar_StatusEffect _array_element) "Burning")
      (bind _structout (Utilities|Struct|SetmembersinAvatar_Struct (Variables|Default|GetAvatarData) (- (.CurrentHealthPoints (Utilities|Struct|BreakAvatar_Struct (Variables|Default|GetAvatarData))) (Math|Float|Round (* (Utilities|Struct|BreakAvatar_BaseStats (.BaseStats (Utilities|Struct|BreakAvatar_Struct (Variables|Default|GetAvatarData)))) 0.1)))))
      (Variables|Default|SetAvatarData _structout)))
  (if (Utilities|Array|ContainsItem (Variables|/Script/Starmark.Actor_GridTile|GetProperties GridTileReference) "Fire")
    (bind _returnvalue (Game|SpawnActorfromClass "/Game/Blueprints/Actor_StatusEffectsLibrary_Blueprint.Actor_StatusEffectsLibrary_Blueprint_C" (Math|Transform|MakeTransform "0, 0, 0") "Undefined" 0 0))
    (bind _returnvalue_2 (Utilities|GetDataTableRow (Variables|/Script/Starmark.Actor_StatusEffectsLibrary|GetStatusEffectsDataTable _returnvalue) "Burning")
      (:then
        (Utilities|Array|Add (Variables|Default|GetCurrentStatusEffectsArray self) _returnvalue_2))
      (:RowNotFound
        (Development|PrintString "Status Effect 'Burning' Not Found")))
    (else
      (bind _structout_2 (Utilities|Struct|SetmembersinAvatar_Struct (Variables|Default|GetAvatarData) (- (.CurrentTileMoves (Utilities|Struct|BreakAvatar_Struct (Variables|Default|GetAvatarData))) 1)))
      (Variables|Default|SetAvatarData _structout_2))))

(event EventTick
  (params (DeltaSeconds :type Float%20%28single-precision%29))
  (bind _actorselectedplane (Variables|Default|GetActorSelectedPlane))
  (bind _returnvalue (Transformation|GetWorldRotation _actorselectedplane))
  (bind (_roll _pitch _yaw) (Math|Rotator|BreakRotator _returnvalue))
  (Transformation|SetWorldRotation _actorselectedplane (Math|Rotator|MakeRotator _roll _pitch (+ _yaw 0.1)) false false)
  (Transformation|SetWorldLocation (Variables|Default|GetAttackTraceCollisionComponent) (Variables|/Script/Starmark.PlayerController_Battle|GetCursorLocationSnappedToGrid (Variables|Default|GetPlayerControllerReference)) false true))

(event EventActorSelectedDynamicMaterialColourUpdate
  (Rendering|Material|SetVectorParameterValue (.AsMaterial%20Instance%20Dynamic (Utilities|Casting|CastToMaterialInstanceDynamic (Rendering|Material|GetMaterial (Variables|Default|GetActorSelectedPlane) 0))) "Colour" (Variables|Default|GetActorSelected_DynamicMaterial_Colour) :!class /Script/Engine.MaterialInstanceDynamic))

(event EventAvatarBeginTileOverlap
  (for _array_element (Variables|Default|GetCurrentStatusEffectsArray)
    (if (Utilities|String|Contains (Utilities|Struct|BreakAvatar_StatusEffect _array_element) "Burning")
      (bind _structout (Utilities|Struct|SetmembersinAvatar_Struct (Variables|Default|GetAvatarData) (- (.CurrentHealthPoints (Utilities|Struct|BreakAvatar_Struct (Variables|Default|GetAvatarData))) (Math|Float|Round (* (Utilities|Struct|BreakAvatar_BaseStats (.BaseStats (Utilities|Struct|BreakAvatar_Struct (Variables|Default|GetAvatarData)))) 0.1)))))
      (Variables|Default|SetAvatarData _structout)))
  (if (Utilities|Array|ContainsItem (Variables|/Script/Starmark.Actor_GridTile|GetProperties (stale Custom|BeginTileOverlap GridTileReference)) "Fire")
    (bind _returnvalue (Game|SpawnActorfromClass "/Game/Blueprints/Actor_StatusEffectsLibrary_Blueprint.Actor_StatusEffectsLibrary_Blueprint_C" (Math|Transform|MakeTransform "0, 0, 0") "Undefined" 0 0))
    (bind _returnvalue_2 (Utilities|GetDataTableRow (Variables|/Script/Starmark.Actor_StatusEffectsLibrary|GetStatusEffectsDataTable _returnvalue) "Burning")
      (:then
        (Utilities|Array|Add (Variables|Default|GetCurrentStatusEffectsArray self) _returnvalue_2))
      (:RowNotFound
        (Development|PrintString "Status Effect 'Burning' Not Found")))
    (else
      (bind _structout_2 (Utilities|Struct|SetmembersinAvatar_Struct (Variables|Default|GetAvatarData) (- (.CurrentTileMoves (Utilities|Struct|BreakAvatar_Struct (Variables|Default|GetAvatarData))) 1)))
      (Variables|Default|SetAvatarData _structout_2))))

(event EventOnLanded
  (params (Hit :type Hit%20Result%20Structure%20%28by%20ref%29))
  (Utilities|FlowControl|Delay 0.2)
  (Class|CharacterPathfinder|AvatarStopMoving true))

(fn ConstructionScript
  (bind _actorselectedplane (Variables|Default|GetActorSelectedPlane))
  (bind _returnvalue (Rendering|Material|CreateDynamicMaterialInstance (Variables|Default|GetActorSelected) :!class /Script/Engine.DecalComponent))
  (Variables|Default|SetActorSelected_DynamicMaterial _returnvalue)
  (Rendering|Material|SetMaterial _actorselectedplane 0 "/Game/Materials/Avatars/selection_ring_MaterialInstance.selection_ring_MaterialInstance")
  (Rendering|Material|CreateDynamicMaterialInstance _actorselectedplane 0 (Rendering|Material|GetMaterial _actorselectedplane 0) "None" :!class /Script/Engine.PrimitiveComponent))